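; Duck actor Blueprint that tracks a point value and a decay state, both of which drop while the duck is left alone.
; Each Decay_Function call subtracts a point and steps DecayState down unless it equals 1, but only while the duck is neither picked up nor falling.
; Points has no lower limit here, and nothing in this graph calls the event.
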(event Custom|Decay_Function
  (if (and (Math|Boolean|Equal(Boolean) (Variables|Default|GetpickedUp) false) (Math|Boolean|Equal(Boolean) (Variables|Default|Getfalling) false))
    (Math|Integer|DecrementInt (Variables|Default|Getpoints)
      (:%20%20
        (if (not (== (Variables|Default|GetdecayState) 1))
          (Math|Integer|DecrementInt (Variables|Default|GetdecayState)))))))

(event EventBeginPlay)

(event Collision|EventActorBeginOverlap
  (params (OtherActor :type Actor%20Object%20Reference)))

(event EventTick
  (params (DeltaSeconds :type Float%20%28single-precision%29)))

(fn ConstructionScript)